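; Audio manager actor that drives the player's suit, breathing and space sounds and plays footstep, jump and airlock door cues.
; Tick moves its audio components to the player, scales suit volume by speed and sets a three-level breathing parameter from remaining oxygen.
; SetAudioInside fades the Space sound and switches between the AudioVolume cached at construction and an outside sound mix.
; One-shot functions play cues at locations, with footstep volume scaled by speed.
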(event EventBeginPlay)

(event Collision|EventActorBeginOverlap
  (params (OtherActor :type Actor%20Object%20Reference)))

(event EventTick
  (params (DeltaSeconds :type Float%20%28single-precision%29))
  (bind _returnvalue (Game|GetPlayerCharacter 0))
  (bind _breathing (Variables|Default|GetBreathing))
  (for _array_element (Utilities|Array|MakeArray (Variables|Default|GetBreathing) (Variables|Default|GetJump) (Variables|Default|GetSuit) (Variables|Default|GetSpace))
    (Transformation|SetWorldLocation _array_element (Transformation|GetActorLocation _returnvalue) false false)
    (Audio|Components|Audio|AdjustVolume (Variables|Default|GetSuit) 0.1 (Math|Float|MapRangeClamped (Math|Vector|VectorLength (Transformation|GetComponentVelocity (Variables|/Script/Engine.Character|GetCapsuleComponent _returnvalue))) 0.0 6e+02 0.0 1.0) "Sin" :!class /Script/Engine.AudioComponent)
    ;[1 1 1] Breathing and oxygen
    (bind _asfirst_person_character (Utilities|Casting|CastToFirstPersonCharacter _returnvalue))
    (Math|Float|CompareFloat (Math|Conversions|ToFloat(Integer) (Variables|/Game/FirstPersonBP/Blueprints/FirstPersonCharacter.FirstPersonCharacter_C|GetCurrentOxygen _asfirst_person_character)) (* (Math|Conversions|ToFloat(Integer) (Variables|/Game/FirstPersonBP/Blueprints/FirstPersonCharacter.FirstPersonCharacter_C|GetMaxOxygen _asfirst_person_character)) 0.25)
      (:>
        (Math|Float|CompareFloat (Math|Conversions|ToFloat(Integer) (Variables|/Game/FirstPersonBP/Blueprints/FirstPersonCharacter.FirstPersonCharacter_C|GetCurrentOxygen _asfirst_person_character)) (* (Math|Conversions|ToFloat(Integer) (Variables|/Game/FirstPersonBP/Blueprints/FirstPersonCharacter.FirstPersonCharacter_C|GetMaxOxygen _asfirst_person_character)) 0.5)
          (:>
            (Effects|Components|ParticleSystem|SetIntParameter _breathing "BreathingOxygen" 0))
          (:==
            (Effects|Components|ParticleSystem|SetIntParameter _breathing "BreathingOxygen" 1 :!label _label))
          (:<
            (goto _label))))
      (:==
        (Effects|Components|ParticleSystem|SetIntParameter _breathing "BreathingOxygen" 2 :!label _label_2))
      (:<
        (goto _label_2)))))

(fn ConstructionScript
  ;[1 1 1] Set AudioVolume
  (bind _outactors (Actor|GetAllActorsOfClass "/Script/Engine.AudioVolume"))
  (for _array_element _outactors
    (Variables|Default|SetAudioVolume _array_element)))

(fn SetAudioInside
  (params (Is%20Inside :type Boolean))
  (bind _audiovolume (Variables|Default|GetAudioVolume))
  (Audio|Components|Audio|AdjustVolume (Variables|Default|GetSpace) 4.0 (Math|Float|Clamp(Float) (Math|Conversions|ToFloat(Boolean) Is%20Inside) 0.05) "Sin" :!class /Script/Engine.AudioComponent)
  (if Is%20Inside
    (Class|GameplayStatics|ClearSoundMixModifiers)
    (Class|AudioVolume|SetEnabled _audiovolume true)
    (else
      (Class|GameplayStatics|ClearSoundMixModifiers)
      (Audio|PushSoundMixModifier "/Game/Audio/SFX/OutsideSoundMix.OutsideSoundMix")
      (Class|AudioVolume|SetEnabled _audiovolume false))))

(fn PlayFootstep
  (bind _returnvalue (Game|GetPlayerCharacter 0))
  (Audio|PlaySoundatLocation "/Game/Audio/SFX/Footsteps/FootstepsCue.FootstepsCue" (Transformation|GetActorLocation _returnvalue) "0, 0, 0" (Math|Float|MapRangeClamped (Math|Vector|VectorLength (Transformation|GetComponentVelocity (Variables|/Script/Engine.Character|GetCapsuleComponent _returnvalue))) 0.0 6e+02 0.0 1.0) 1.0 0.0 0 0 0))

(fn PlayJump
  (Audio|PlaySoundatLocation "/Game/Audio/SFX/Jump/JumpCue.JumpCue" (Transformation|GetActorLocation (Game|GetPlayerCharacter 0)) "0, 0, 0" 1.0 1.0 0.0 0 0 0))

(fn PlayAirlockDoorClick
  (params (DoorLocation :type Vector))
  (Audio|PlaySoundatLocation "/Game/Audio/SFX/Airlock/AirlockDoorClickCue.AirlockDoorClickCue" DoorLocation "0, 0, 0" 1.0 1.0 0.0 0 0 0))