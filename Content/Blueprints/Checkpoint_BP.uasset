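; One-shot checkpoint actor that saves game progress when its trigger volume is first overlapped.
; On overlap it loads the "check" SavePoint save, or creates one if none exists, then passes it to SaveF and destroys itself.
; SaveF writes the player's transform and oxygen plus the FollowPlayer monster's transform to that slot.
; The overlapping actor is not filtered, and older inline save nodes remain unconnected.
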(event OnComponentBeginOverlap(Trigger)
  (params (OverlappedComponent :type Primitive%20Component%20Object%20Reference) (OtherActor :type Actor%20Object%20Reference) (OtherComp :type Primitive%20Component%20Object%20Reference) (OtherBodyIndex :type Integer) (bFromSweep :type Boolean) (SweepResult :type Hit%20Result%20Structure%20%28by%20ref%29))
  (if (not (Variables|Default|GetIsTrigger))
    (Variables|Default|SetIsTrigger true)
    (Development|PrintString "Checkpoint Reached!")
    (bind _returnvalue (SaveGame|DoesSaveGameExist "check"))
    (if _returnvalue
      (bind _returnvalue_2 (SaveGame|LoadGamefromSlot "check"))
      (bind _assave_point (Utilities|Casting|CastToSavePoint _returnvalue_2))
      (CallFunction|SaveF _assave_point)
      (Actor|DestroyActor)
      (else
        (bind _returnvalue_3 (SaveGame|CreateSaveGameObject "/Game/Blueprints/SavePoint.SavePoint_C"))
        (CallFunction|SaveF _returnvalue_3)
        (Actor|DestroyActor)))))

(event EventBeginPlay)

(event Collision|EventActorBeginOverlap
  (params (OtherActor :type Actor%20Object%20Reference)))

(event EventTick
  (params (DeltaSeconds :type Float%20%28single-precision%29)))

(fn ConstructionScript)

(fn SaveF
  (params (SavePoint :type Save%20Point%20Object%20Reference))
  (bind _returnvalue (Actor|GetActorOfClass "/Game/FirstPersonBP/Blueprints/FirstPersonCharacter.FirstPersonCharacter_C"))
  (Variables|/Game/Blueprints/SavePoint.SavePoint_C|SetPlayerTransform SavePoint (Math|Transform|MakeTransform (Transformation|GetActorLocation _returnvalue) (Transformation|GetActorRotation _returnvalue) (Transformation|GetActorScale3D _returnvalue)))
  (Variables|/Game/Blueprints/SavePoint.SavePoint_C|SetCurrentOxygen SavePoint (Variables|/Game/FirstPersonBP/Blueprints/FirstPersonCharacter.FirstPersonCharacter_C|GetCurrentOxygen _returnvalue))
  (bind _returnvalue_2 (Actor|GetActorOfClass "/Game/FirstPerson/Characters/Monster/FollowPlayer.FollowPlayer_C"))
  (Variables|/Game/Blueprints/SavePoint.SavePoint_C|SetMonsterTransform SavePoint (Math|Transform|MakeTransform (Transformation|GetActorLocation _returnvalue_2) (Transformation|GetActorRotation _returnvalue_2) (Transformation|GetActorScale3D _returnvalue_2)))
  (SaveGame|SaveGametoSlot SavePoint "check"))