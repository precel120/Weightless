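; A one-way moving platform that carries the first-person character from its start position to an EndPoint component.
; Actor overlap stores the character, flags it as touching a wall, plays a jump sound and stops its movement.
; Box overlap plays the Platform_Move timeline, whose updates also play Player_Move; both sweep platform and player along the same lerped path.
; The construction script finds the AudioManager; collision-toggle nodes are unwired.
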(event OnComponentBeginOverlap(Box)
  (params (OverlappedComponent :type Primitive%20Component%20Object%20Reference) (OtherActor :type Actor%20Object%20Reference) (OtherComp :type Primitive%20Component%20Object%20Reference) (OtherBodyIndex :type Integer) (bFromSweep :type Boolean) (SweepResult :type Hit%20Result%20Structure%20%28by%20ref%29))
  (Utilities|Casting|CastToFirstPersonCharacter OtherActor)
  (bind _newtrack_0 (Timeline|Platform_Move Play)
    (:Update
      (Transformation|SetWorldLocation (Variables|Default|Getplatform) (Math|Vector|Lerp(Vector) (Variables|Default|Getstart_location) (Variables|Default|Getend_location) _newtrack_0) true false)
      (bind _newtrack_0_2 (Timeline|Player_Move Play)
        (:Update
          (Transformation|SetWorldLocation (Variables|/Script/Engine.Actor|GetRootComponent (Variables|Default|GetFirstPersonRef)) (Math|Vector|Lerp(Vector) (Variables|Default|Getstart_location) (Variables|Default|Getend_location) _newtrack_0_2) true false))))))

(event EventBeginPlay
  (Variables|Default|Setstart_location (Transformation|GetWorldLocation (Variables|Default|Getplatform)))
  (Variables|Default|Setend_location (Transformation|GetWorldLocation (Variables|Default|Getend_point)))
  (Variables|Default|Setstart_player (Transformation|GetWorldLocation (Variables|/Script/Engine.Character|GetCapsuleComponent (Variables|Default|GetFirstPersonRef))))
  (Components|Timeline|SetPlayRate (Variables|Default|GetPlatform_Move) (Variables|Default|Getplayrate))
  (Components|Timeline|SetPlayRate (Variables|Default|GetPlayer_Move) (Variables|Default|Getplayrate)))

(event Collision|EventActorBeginOverlap
  (params (OtherActor :type Actor%20Object%20Reference))
  (bind _asfirst_person_character (Utilities|Casting|CastToFirstPersonCharacter OtherActor))
  (bind _output_get (Variables|Default|SetFirstPersonRef _asfirst_person_character))
  (Variables|/Game/FirstPersonBP/Blueprints/FirstPersonCharacter.FirstPersonCharacter_C|SetIsTouchingWall? (Variables|Default|GetFirstPersonRef) true)
  (Default|PlayJump (Variables|Default|GetAudioManager))
  (Components|Movement|StopMovementImmediately (Variables|/Script/Engine.Character|GetCharacterMovement (Variables|Default|GetFirstPersonRef))))

(event EventTick
  (params (DeltaSeconds :type Float%20%28single-precision%29)))

(fn ConstructionScript
  ;[1 1 1] Set AudioManager
  (bind _outactors (Actor|GetAllActorsOfClass "/Game/Audio/Blueprints/AudioManager.AudioManager_C"))
  (for _array_element _outactors
    (Variables|Default|SetAudioManager _array_element)))