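; Trigger volume that puts the first-person character into the no-gravity state while marking them as no longer outside.
; On BeginPlay it caches the level's AudioManager.
; When the character begins overlapping OxygenBox, it sets the no-gravity and touching-wall flags, prints a debug message and clears the outside and returning-from-outside flags.
; It then passes the cleared outside flag to the AudioManager's SetAudioInside.
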(event OnComponentBeginOverlap(OxygenBox)
  (params (OverlappedComponent :type Primitive%20Component%20Object%20Reference) (OtherActor :type Actor%20Object%20Reference) (OtherComp :type Primitive%20Component%20Object%20Reference) (OtherBodyIndex :type Integer) (bFromSweep :type Boolean) (SweepResult :type Hit%20Result%20Structure%20%28by%20ref%29))
  (Utilities|FlowControl|Sequence
    (:then_0
      (bind _asfirst_person_character (Utilities|Casting|CastToFirstPersonCharacter OtherActor))
      (Variables|Default|SetFirstPersonRef _asfirst_person_character)
      (Variables|/Game/FirstPersonBP/Blueprints/FirstPersonCharacter.FirstPersonCharacter_C|SetIsNoGravity? (Variables|Default|GetFirstPersonRef) true)
      (Development|PrintString "Hello")
      (Variables|/Game/FirstPersonBP/Blueprints/FirstPersonCharacter.FirstPersonCharacter_C|SetIsTouchingWall? (Variables|Default|GetFirstPersonRef) true))
    (:then_1
      (bind _asfirst_person_character_2 (Utilities|Casting|CastToFirstPersonCharacter OtherActor))
      (Variables|Default|SetFirstPersonRef _asfirst_person_character_2)
      (Variables|/Game/FirstPersonBP/Blueprints/FirstPersonCharacter.FirstPersonCharacter_C|SetComingBackFromOutside (Variables|Default|GetFirstPersonRef) false)
      (bind _output_get (Variables|/Game/FirstPersonBP/Blueprints/FirstPersonCharacter.FirstPersonCharacter_C|SetIsOutside? (Variables|Default|GetFirstPersonRef) false))
      (Default|SetAudioInside (Variables|Default|GetAudioManager) _output_get))))

(event EventBeginPlay
  ;[1 1 1] Set AudioManager
  (bind _outactors (Actor|GetAllActorsOfClass "/Game/Audio/Blueprints/AudioManager.AudioManager_C"))
  (for _array_element _outactors
    (Variables|Default|SetAudioManager _array_element)))

(event Collision|EventActorBeginOverlap
  (params (OtherActor :type Actor%20Object%20Reference)))

(event EventTick
  (params (DeltaSeconds :type Float%20%28single-precision%29)))

(fn ConstructionScript)