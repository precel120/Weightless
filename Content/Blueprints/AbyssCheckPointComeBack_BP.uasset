(event OnComponentBeginOverlap(Abyss)
  (params (OverlappedComponent :type Primitive%20Component%20Object%20Reference) (OtherActor :type Actor%20Object%20Reference) (OtherComp :type Primitive%20Component%20Object%20Reference) (OtherBodyIndex :type Integer) (bFromSweep :type Boolean) (SweepResult :type Hit%20Result%20Structure%20%28by%20ref%29))
  (bind _returnvalue (SaveGame|DoesSaveGameExist "check"))
  (if _returnvalue
    (bind _asfirst_person_character (Utilities|Casting|CastToFirstPersonCharacter OtherActor))
    (Variables|Default|SetFirstPersonRef _asfirst_person_character)
    (Variables|/Game/FirstPersonBP/Blueprints/FirstPersonCharacter.FirstPersonCharacter_C|SetIsNoGravity? (Variables|Default|GetFirstPersonRef) (not (Variables|/Game/FirstPersonBP/Blueprints/FirstPersonCharacter.FirstPersonCharacter_C|GetIsNoGravity? (Variables|Default|GetFirstPersonRef))))
    (Development|PrintString "You went into the abbys! Come Back!")
    (bind _returnvalue_2 (SaveGame|LoadGamefromSlot "check"))
    (bind _assave_point (Utilities|Casting|CastToSavePoint _returnvalue_2))
    (bind _asfirst_person_character_2 (Utilities|Casting|CastToFirstPersonCharacter (Game|GetPlayerCharacter 0)))
    (Transformation|SetActorLocation _asfirst_person_character_2 (Variables|/Game/Blueprints/SavePoint.SavePoint_C|GetPlayerLocation _assave_point) false false)
    (else
      (Development|PrintString "You Died!"))))

(event EventBeginPlay)

(event Collision|EventActorBeginOverlap
  (params (OtherActor :type Actor%20Object%20Reference)))

(event EventTick
  (params (DeltaSeconds :type Float%20%28single-precision%29)))

(fn ConstructionScript)