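; A moving box that slides back and forth along its X axis and catches the first-person player on overlap.
; MoveLeftRight chains latent MoveComponentTo calls, using MoveLeft and MoveRight for targets, then calls itself to loop from BeginPlay.
; Actor overlap stores the player, flags wall contact, stops movement and plays a jump sound through the AudioManager found at construction.
; Cube overlap snaps the stored player's root onto the cube.
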(event OnComponentBeginOverlap(Cube)
  (params (OverlappedComponent :type Primitive%20Component%20Object%20Reference) (OtherActor :type Actor%20Object%20Reference) (OtherComp :type Primitive%20Component%20Object%20Reference) (OtherBodyIndex :type Integer) (bFromSweep :type Boolean) (SweepResult :type Hit%20Result%20Structure%20%28by%20ref%29))
  (Transformation|AttachComponentToComponent (Variables|/Script/Engine.Actor|GetRootComponent (Variables|Default|GetFirstPersonRef)) (Variables|Default|GetCube) "None" "SnapToTarget" "SnapToTarget" "KeepRelative" true)
  (Variables|Default|SetisAttached true))

(event Custom|MoveLeftRight
  (Utilities|FlowControl|Sequence
    (:then_0
      (bind (_newposition _newrotation) (CallFunction|MoveLeft (Variables|Default|GetCube)))
      (Components|MoveComponentTo (Variables|Default|GetCube) _newposition (Math|Conversions|RotationFromXVector _newrotation) false false (Variables|Default|GetMovingTime) false)
      (bind (_newposition_2 _newrotation_2) (CallFunction|MoveRight (Variables|Default|GetCube)))
      (Components|MoveComponentTo (Variables|Default|GetCube) _newposition_2 (Math|Conversions|RotationFromXVector _newrotation_2) false false (Variables|Default|GetMovingTime) false)
      (CallFunction|MoveLeftRight))))

(event EventBeginPlay
  (CallFunction|MoveLeftRight)
  (if (Variables|Default|GetisAttached)
    (Collision|SetCollisionEnabled (Variables|Default|GetCube) "NoCollision")
    (else
      (Collision|SetCollisionEnabled (Variables|Default|GetCube) "QueryAndPhysics"))))

(event Collision|EventActorBeginOverlap
  (params (OtherActor :type Actor%20Object%20Reference))
  (bind _asfirst_person_character (Utilities|Casting|CastToFirstPersonCharacter OtherActor))
  (bind _output_get (Variables|Default|SetFirstPersonRef _asfirst_person_character))
  (Variables|/Game/FirstPersonBP/Blueprints/FirstPersonCharacter.FirstPersonCharacter_C|SetIsTouchingWall? (Variables|Default|GetFirstPersonRef) true)
  (Default|PlayJump (Variables|Default|GetAudioManager))
  (Components|Movement|StopMovementImmediately (Variables|/Script/Engine.Character|GetCharacterMovement (Variables|Default|GetFirstPersonRef))))

(fn ConstructionScript
  ;[1 1 1] Set AudioManager
  (bind _outactors (Actor|GetAllActorsOfClass "/Game/Audio/Blueprints/AudioManager.AudioManager_C"))
  (for _array_element _outactors
    (Variables|Default|SetAudioManager _array_element)))

(fn MoveLeft
  (params (Cube :type Static%20Mesh%20Component%20Object%20Reference))
  (bind _relativelocation (Variables|/Script/Engine.SceneComponent|GetRelativeLocation Cube))
  (return (Math|Vector|MakeVector (- (.x _relativelocation) (Variables|Default|GetMoveDistance)) (.y _relativelocation) (.z _relativelocation)) (Math|Rotator|GetRotationXVector (Variables|/Script/Engine.SceneComponent|GetRelativeRotation Cube))))

(fn MoveRight
  (params (Cube :type Static%20Mesh%20Component%20Object%20Reference))
  (bind _relativelocation (Variables|/Script/Engine.SceneComponent|GetRelativeLocation Cube))
  (return (Math|Vector|MakeVector (+ (.x _relativelocation) (Variables|Default|GetMoveDistance)) (.y _relativelocation) (.z _relativelocation)) (Math|Rotator|GetRotationXVector (Variables|/Script/Engine.SceneComponent|GetRelativeRotation Cube))))